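; Player-controlled escape pod that flies on physics, steered with thruster components.
; On BeginPlay it throws the cylinder body downward and sets it tumbling with a large force and torque.
; Axis inputs set thruster strength through helper functions: diagonal top/bottom pairs rotate the pod, while side thrusters translate it at double the multiplier.
; The main thruster input also scales a light's intensity with thrust.
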(event Collision|EventActorBeginOverlap
  (params (OtherActor :type Actor%20Object%20Reference)))

(event EventTick
  (params (DeltaSeconds :type Float%20%28single-precision%29)))

(event EventBeginPlay
  (bind _cylinder (Variables|Default|GetCylinder))
  (Physics|AddForce _cylinder "0, 0,-30000000.000000" "None" false)
  (Class|PrimitiveComponent|AddTorque _cylinder "0.000000,60000000.000000,60000000.000000" "None" false))

(event Input|AxisEvents|InputAxisRotateLeft
  (params (AxisValue :type Float%20%28single-precision%29))
  (CallFunction|RotateThrust (Variables|Default|GetTRThruster) (Variables|Default|GetBLThruster) AxisValue))

(event Input|AxisEvents|InputAxisRotateRight
  (params (AxisValue :type Float%20%28single-precision%29))
  (CallFunction|RotateThrust (Variables|Default|GetTLThruster) (Variables|Default|GetBRThruster) AxisValue))

(event Input|AxisEvents|InputAxisMoveLeft
  (params (AxisValue :type Float%20%28single-precision%29))
  (CallFunction|TranslateThrust (Variables|Default|GetTransLThruster) AxisValue))

(event Input|AxisEvents|InputAxisMoveRight
  (params (AxisValue :type Float%20%28single-precision%29))
  (CallFunction|TranslateThrust (Variables|Default|GetTransRThruster) AxisValue))

(event Input|AxisEvents|InputAxisMainThruster
  (params (AxisValue :type Float%20%28single-precision%29))
  (Variables|/Script/Engine.PhysicsThrusterComponent|SetThrustStrength (Variables|Default|GetMainThruster) (* AxisValue 3e+05))
  (Rendering|Components|Light|SetIntensity (Variables|Default|GetMainThrusterLight) (* AxisValue 5e+04)))

(fn ConstructionScript)

(fn RotateThrust
  (params (Top%20Thruster :type Physics%20Thruster%20Component%20Object%20Reference) (Bottom%20Thruster :type Physics%20Thruster%20Component%20Object%20Reference) (Value :type Float%20%28single-precision%29))
  (bind _thrustmultiplier (Variables|Default|GetThrustMultiplier))
  (bind _returnvalue (* Value _thrustmultiplier))
  (Variables|/Script/Engine.PhysicsThrusterComponent|SetThrustStrength Top%20Thruster _returnvalue)
  (Variables|/Script/Engine.PhysicsThrusterComponent|SetThrustStrength Bottom%20Thruster _returnvalue))

(fn TranslateThrust
  (params (Translate%20Thruster :type Physics%20Thruster%20Component%20Object%20Reference) (Value :type Float%20%28single-precision%29))
  (Variables|/Script/Engine.PhysicsThrusterComponent|SetThrustStrength Translate%20Thruster (* Value (* (Variables|Default|GetThrustMultiplier) 2.0))))