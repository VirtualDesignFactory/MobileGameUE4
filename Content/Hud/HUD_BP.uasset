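; HUD Blueprint that adds the Hud_WBP widget to the viewport and marks landing zones on screen until LandingComplete is set.
; BeginPlay gathers all LandingZone_BP actors once and caches them.
; Each DrawHUD calls LandingGamePlay, which projects every cached zone to screen space and draws a translucent blue square with a "Landing Zone" label.
; The square is a placeholder for a sprite sheet, and the projection result is not checked for visibility.
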(event EventBeginPlay
  (bind _returnvalue (UserInterface|CreateWidget "/Game/Hud/Hud_WBP.Hud_WBP_C"))
  (UserInterface|Viewport|AddtoViewport _returnvalue 0)
  (bind _outactors (Actor|GetAllActorsOfClass "/Game/EscapePod/LandingZone_BP.LandingZone_BP_C"))
  (Variables|Default|SetLandingZoneReference _outactors)
  (Development|PrintString "Gethered landing zones"))

(event Collision|EventActorBeginOverlap
  (params (OtherActor :type Actor%20Object%20Reference)))

(event EventTick
  (params (DeltaSeconds :type Float%20%28single-precision%29)))

(event EventDrawHUD
  (params (SizeX :type Integer) (SizeY :type Integer))
  (if (not (Variables|Default|GetLandingComplete?))
    (CallFunction|LandingGamePlay)))

(fn ConstructionScript)

(fn LandingGamePlay
  (for _array_element (Variables|Default|GetLandingZoneReference)
    ;[1 1 1] Replace with a sprite sheet
    (HUD|DrawRect "(R=0.045186,G=0.223228,B=0.938686,A=0.498039)" (- (.X (Math|Vector2D|BreakVector2D (.ScreenPosition (Class|GameplayStatics|ProjectWorldtoScreen (Game|GetPlayerController 0) (Transformation|GetActorLocation _array_element) false)))) 12.0) (- (.Y (Math|Vector2D|BreakVector2D (.ScreenPosition (Class|GameplayStatics|ProjectWorldtoScreen (Game|GetPlayerController 0) (Transformation|GetActorLocation _array_element) false)))) 12.0) 25.0 25.0)
    (HUD|DrawText "Landing Zone" "(R=0.045186,G=0.223228,B=0.938686,A=0.500000)" (- (.X (Math|Vector2D|BreakVector2D (.ScreenPosition (Class|GameplayStatics|ProjectWorldtoScreen (Game|GetPlayerController 0) (Transformation|GetActorLocation _array_element) false)))) 5e+01) (- (.Y (Math|Vector2D|BreakVector2D (.ScreenPosition (Class|GameplayStatics|ProjectWorldtoScreen (Game|GetPlayerController 0) (Transformation|GetActorLocation _array_element) false)))) 3e+01) "/Game/Fonts/Slider.Slider" 1.0 false)))